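; BP_PickUp is a collectible whose static mesh spins every tick and adds one to the collecting actor's Score.
; On overlap with an actor that passes the cast, it creates a WG_PickUp widget and destroys the mesh.
; A timeline moves the widget from the collector's projected screen position toward a fixed top-left point.
; When it finishes, the score increments, the widget is removed and the pickup destroys itself.
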(event OnComponentBeginOverlap(StaticMesh)
  (params (OverlappedComponent :type Primitive%20Component%20Object%20Reference) (OtherActor :type Actor%20Object%20Reference) (OtherComp :type Primitive%20Component%20Object%20Reference) (OtherBodyIndex :type Integer) (bFromSweep :type Boolean) (SweepResult :type Hit%20Result%20Structure%20%28by%20ref%29))
  (bind _asside_scroller_character (Utilities|Casting|CastTo OtherActor))
  (bind _returnvalue (UserInterface|CreateWidget "/Game/Blueprints/Hud/WG_PickUp.WG_PickUp_C"))
  (bind _output_get (Variables|Default|SetWG_PU _returnvalue))
  (UserInterface|Viewport|AddtoViewport _output_get 0)
  (Components|DestroyComponent (Variables|Default|GetStaticMesh))
  (Components|Timeline|SetPlayRate (Variables|Default|GetPos) (Variables|Default|GetSpriteSpeed))
  (bind _newtrack_0 (Timeline|Pos PlayFromStart)
    (:Update
      (Class|UserWidget|SetPositioninViewport (Variables|Default|GetWG_PU) (Math|Vector2D|MakeVector2D (Math|Float|Lerp (.x (.ScreenPosition (Class|GameplayStatics|ProjectWorldtoScreen (Game|GetPlayerController 0) (Transformation|GetActorLocation _asside_scroller_character) true))) 4e+01 _newtrack_0) (Math|Float|Lerp (.y (.ScreenPosition (Class|GameplayStatics|ProjectWorldtoScreen (Game|GetPlayerController 0) (Transformation|GetActorLocation _asside_scroller_character) true))) 4e+01 _newtrack_0)) true))
    (:Finished
      (Math|Integer|IncrementInt (Variables|Default|GetScore _asside_scroller_character)
        (:%20%20
          (Widget|RemovefromParent (Variables|Default|GetWG_PU))
          (Actor|DestroyActor))))))

(event EventBeginPlay)

(event Collision|EventActorBeginOverlap
  (params (OtherActor :type Actor%20Object%20Reference)))

(event EventTick
  (params (DeltaSeconds :type Float%20%28single-precision%29))
  (bind _staticmesh (Variables|Default|GetStaticMesh)
    (:then
      (Transformation|AddWorldRotation _staticmesh (Math|Rotator|MakeRotator 0.0 0.0 (Variables|Default|GetMeshRotation)) false false))
    (:else)))

(fn ConstructionScript)