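; Controller Blueprint that turns the SpeedCart and SlowCart inputs into a bounded OffSet value, presumably for cart movement.
; Each Tick, holding SpeedCart raises OffSet by an accelerating Speed, while SlowCart lowers it by an accelerating Slow, with SpeedCart taking priority.
; Both step sizes grow multiplicatively and ease back linearly to a minimum when inactive.
; BeginPlay sets game-only input, Slow prints every frame, and nothing here applies OffSet.
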(event EventBeginPlay
  (Input|SetInputModeGameOnly (Game|GetPlayerController 0)))

(event EventTick
  (params (DeltaSeconds :type Float%20%28single-precision%29))
  (Development|PrintString (Utilities|String|ToString(Float) (Variables|Default|GetSlow)))
  (if (Variables|Default|GetInputDown)
    (Variables|Default|SetSlow 3.0)
    (Variables|Default|SetOffSet (Math|Float|Clamp(Float) (+ (Variables|Default|GetOffSet) (Variables|Default|GetSpeed)) -5e+02 5e+02))
    (Variables|Default|SetSpeed (Math|Float|Clamp(Float) (* (Variables|Default|GetSpeed) 1.02) 0.0 1e+01))
    (else
      (Variables|Default|SetSpeed (Math|Float|Clamp(Float) (- (Variables|Default|GetSpeed) 0.1) 3.0 1e+01))
      (if (Variables|Default|GetInputDown2)
        (Variables|Default|SetOffSet (Math|Float|Clamp(Float) (- (Variables|Default|GetOffSet) (Variables|Default|GetSlow)) -5e+02 5e+02))
        (Variables|Default|SetSlow (Math|Float|Clamp(Float) (* (Variables|Default|GetSlow) 1.02) 0.0 1e+01))
        (else
          (Variables|Default|SetSlow (Math|Float|Clamp(Float) (- (Variables|Default|GetSlow) 0.1) 3.0 1e+01)))))))

(event Input|ActionEvents|InputActionSpeedCart
  (params (Key :type Key%20Structure :default "None"))
  (:Pressed
    (Variables|Default|SetInputDown true))
  (:Released
    (Variables|Default|SetInputDown false)))

(event Input|ActionEvents|InputActionSlowCart
  (params (Key :type Key%20Structure :default "None"))
  (:Pressed
    (Variables|Default|SetInputDown2 true))
  (:Released
    (Variables|Default|SetInputDown2 false)))

(fn ConstructionScript)