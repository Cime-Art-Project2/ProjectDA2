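; Player cart that rides spline rails and can jump off them to fly free until it enters another rail.
; On a rail, Tick moves and orients it along the tangent, easing speed faster downhill and slower uphill.
; Jump detaches only on flatter track; off-rail, it integrates velocity and gravity with swept moves, and rail ends pass on exit velocity.
; A debug widget, prints and U-key camera zoom toggle round it out.
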(event Custom|OnEnterRail
  (params (Rail :type Bp%20Spline%20Jump%20N%20Switch%20Object%20Reference))
  (Development|PrintString "Enter rail")
  (bind _output_get (Variables|Default|SetAttachedSpline Rail))
  (CallFunction|StopMovement false)
  (Transformation|SetActorLocation (.LocationWithOffset (Default|GetRailData _output_get "World")) false true))

(event Custom|OnReachedRailEnd
  (params (ExitVelocity :type Vector))
  (Development|PrintString "Reached end of rail" true true "(R=1.000000,G=0.442751,B=0.000000,A=1.000000)")
  (Variables|Default|SetAttachedSpline 0)
  (Variables|Physics|SetCartVelocity ExitVelocity))

(event EventTick
  (params (DeltaSeconds :type Float%20%28single-precision%29))
  (bind _attachedspline (Variables|Default|GetAttachedSpline))
  (bind _cartspeed (Variables|Physics|GetCartSpeed))
  (bind (_location _locationwithoffset _tangent _upvector) (Default|GetRailData _attachedspline "World"))
  (bind _returnvalue (Math|Vector|Normalize _tangent))
  (Physics|ConsumeVelocity DeltaSeconds)
  (CallFunction|AdjustCamera DeltaSeconds 4.0)
  (Utilities|IsValid _attachedspline
    (:Is%20Valid
      (Development|PrintString (Utilities|String|Append "RailTangent : " (Utilities|String|ToString(Vector) (Math|Vector|MakeVector (.x _returnvalue) (.y _returnvalue) (.z _returnvalue)))) true false "(R=1.000000,G=0.270337,B=0.000000,A=1.000000)" (Utilities|Time|GetWorldDeltaSeconds))
      (Variables|Physics|SetMomentumSpeed (Math|Interpolation|FInterpTo (Variables|Physics|GetMomentumSpeed) (Math|Float|MapRangeClamped (.z _returnvalue) -1.0 1.0 (* _cartspeed 1.5) (* _cartspeed 0.5)) (Utilities|Time|GetWorldDeltaSeconds) 4.0))
      (Transformation|SetActorLocation (+ _locationwithoffset (* _tangent (* (/ (Math|Interpolation|FInterpTo (Variables|Physics|GetMomentumSpeed) (Math|Float|MapRangeClamped (.z _returnvalue) -1.0 1.0 (* _cartspeed 1.5) (* _cartspeed 0.5)) (Utilities|Time|GetWorldDeltaSeconds) 4.0) (Variables|Physics|GetCartFriction)) (Utilities|Time|GetWorldDeltaSeconds)))) false true)
      (Transformation|SetActorRotation (Math|Rotator|MakeRotfromXZ _tangent _upvector)))))

(event EventBeginPlay
  (bind _returnvalue (UserInterface|CreateWidget "/Game/Widgets/WB_DebugData.WB_DebugData_C"))
  (UserInterface|Viewport|AddtoViewport _returnvalue 0))

(event Input|KeyboardEvents|U
  (params (Key :type Key%20Structure :default "None"))
  (:Pressed
    (Utilities|FlowControl|FlipFlop
      (:A
        (Variables|Camera|SetCameraDistance 1.6e+03))
      (:B
        (Variables|Camera|SetCameraDistance 8e+02)))))

(event Input|ActionEvents|InputActionJump
  (params (Key :type Key%20Structure :default "None"))
  (bind _cartspeed (Variables|Physics|GetCartSpeed))
  (:Pressed
    (Utilities|IsValid (Variables|Default|GetAttachedSpline)
      (:Is%20Valid
        (if (<= (Math|Float|Absolute(Float) (.z (Math|Vector|Normalize (.Tangent (Default|GetRailData (Variables|Default|GetAttachedSpline) "World"))))) 0.55)
          (CallFunction|StopMovement false)
          (Variables|Physics|SetCartVelocity (Math|Vector|MakeVector (.x (* (.Tangent (Default|GetRailData (Variables|Default|GetAttachedSpline) "World")) (* _cartspeed 0.25))) (.y (* (.Tangent (Default|GetRailData (Variables|Default|GetAttachedSpline) "World")) (* _cartspeed 0.25))) (* _cartspeed (* (.z (Variables|Physics|GetGravityDirection)) -0.35))))
          (Variables|Default|SetAttachedSpline 0))))))

(fn ConstructionScript
  (Variables|/Script/Engine.SpringArmComponent|SetTargetArmLength (Variables|Default|GetSpringArm) (Variables|Camera|GetCameraDistance)))

(fn ConsumeVelocity
  (params (DeltaTime :type Float%20%28single-precision%29))
  (LocalVariables|SetCurLoc (Transformation|GetActorLocation))
  (Variables|Physics|SetCartVelocity (Math|Vector|SelectVector "0, 0, 0" (+ (Variables|Physics|GetCartVelocity) (* (Variables|Physics|GetGravityDirection) (* DeltaTime (Variables|Physics|GetGravityForce)))) (Utilities|IsValid (Variables|Default|GetAttachedSpline))))
  (Transformation|SetActorLocation (+ (Transformation|GetActorLocation) (* (Variables|Physics|GetCartVelocity) DeltaTime)) true false))

(fn AdjustCamera
  (params (DeltaTime :type Float%20%28single-precision%29) (InterpSpeed :type Float%20%28single-precision%29))
  (bind _springarm (Variables|Default|GetSpringArm))
  (Variables|/Script/Engine.SpringArmComponent|SetTargetArmLength _springarm (Math|Interpolation|FInterpTo (Variables|/Script/Engine.SpringArmComponent|GetTargetArmLength _springarm) (Variables|Camera|GetCameraDistance) DeltaTime InterpSpeed)))

(fn StopMovement
  (params (StopGravity :type Boolean))
  (Variables|Physics|SetCartVelocity "0, 0, 0")
  (Variables|Physics|SetGravityForce (Math|Float|SelectFloat 0.0 2.0 StopGravity)))