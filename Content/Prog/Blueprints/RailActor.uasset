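; Spline-based rail actor that a CartPawn enters and rides until it reaches the end.
; The construction script builds a spline mesh for each segment between points.
; On Tick, a CartReceiver component snaps to the spline point closest to the player; overlapping it calls OnEnterRail on the cart.
; GetRailData samples the spline at the receiver, and Tick passes the tangent to OnReachedRailEnd when the cart nears the last point.
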(event OnComponentBeginOverlap(CartReceiver)
  (params (OverlappedComponent :type Primitive%20Component%20Object%20Reference) (OtherActor :type Actor%20Object%20Reference) (OtherComp :type Primitive%20Component%20Object%20Reference) (OtherBodyIndex :type Integer) (bFromSweep :type Boolean) (SweepResult :type Hit%20Result%20Structure%20%28by%20ref%29))
  (bind _ascart_pawn (Utilities|Casting|CastToCartPawn OtherActor))
  (Default|OnEnterRail _ascart_pawn self))

(event EventTick
  (params (DeltaSeconds :type Float%20%28single-precision%29))
  (bind _returnvalue (Game|Player|GetPlayerPawn 0))
  (bind _spline (Variables|Default|GetSpline))
  (bind _spline_2 (Variables|Default|GetSpline))
  (bind _returnvalue_2 (Transformation|GetActorLocation _returnvalue))
  (Transformation|SetWorldLocationAndRotation (Variables|Default|GetCartReceiver) (Spline|FindLocationClosesttoWorldLocation _spline _returnvalue_2 "World") (Class|SplineComponent|FindRotationClosesttoWorldLocation _spline _returnvalue_2 "World") false true)
  (if (< (- (Math|Vector|Distance(Vector) (Spline|GetLocationatSplinePoint _spline_2 (- (Spline|GetNumberOfSplinePoints _spline_2) 1) "World") (Transformation|GetActorLocation (CallFunction|GetCartPawn))) (Variables|Default|GetCartOffset)) 2e+01)
    (Default|OnReachedRailEnd (CallFunction|GetCartPawn) (* (.Tangent (CallFunction|GetRailData "World")) 1.0))))

(fn ConstructionScript
  (bind _spline (Variables|Default|GetSpline))
  (for _index (range 0 (- (Spline|GetNumberOfSplinePoints (Variables|Default|GetSpline)) 2))
    (bind _returnvalue (AddComponent|AddSplineMeshComponent false))
    (Components|StaticMesh|SetStaticMesh _returnvalue (Variables|Default|GetStaticMesh))
    (Transformation|AttachComponentToComponent _returnvalue (Variables|Default|GetDefaultSceneRoot) "None" "KeepRelative" "KeepRelative" "KeepRelative" true)
    (SplineMesh|SetStartandEnd _returnvalue (.Location (Spline|GetLocationandTangentatSplinePoint _spline _index "Local")) (.Tangent (Spline|GetLocationandTangentatSplinePoint _spline _index "Local")) (.Location (Spline|GetLocationandTangentatSplinePoint _spline (+ _index 1) "Local")) (.Tangent (Spline|GetLocationandTangentatSplinePoint _spline (+ _index 1) "Local")) true :!class /Script/Engine.SplineMeshComponent)))

(fn GetRailData
  (params (CoordinateSpace :type ESplineCoordinateSpace%20Enum :default "World"))
  (bind _spline (Variables|Default|GetSpline))
  (bind _cartreceiver (Variables|Default|GetCartReceiver))
  (bind _returnvalue (Transformation|GetWorldLocation _cartreceiver))
  (bind _returnvalue_2 (Spline|FindLocationClosesttoWorldLocation _spline _returnvalue CoordinateSpace))
  (bind _returnvalue_3 (Class|SplineComponent|FindUpVectorClosesttoWorldLocation _spline _returnvalue CoordinateSpace))
  (return _returnvalue_2 (+ _returnvalue_2 (* _returnvalue_3 (Variables|Default|GetCartOffset))) (Class|SplineComponent|FindTangentClosesttoWorldLocation _spline _returnvalue CoordinateSpace) _returnvalue_3 (Class|SplineComponent|FindRotationClosesttoWorldLocation _spline _returnvalue CoordinateSpace)))