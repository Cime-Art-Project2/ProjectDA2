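; BP_Mort is a trigger box actor that ends the game when the player's CartPawn overlaps it.
; On the first overlap only, it drops the cart's spring arm camera lag speed to near zero and sets the cart speed to a fixed value.
; It then shows the WG_EndGame widget, initialized with its Win variable, and switches input to UI only with a visible mouse cursor.
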(event OnComponentBeginOverlap(Box)
  (params (OverlappedComponent :type Primitive%20Component%20Object%20Reference) (OtherActor :type Actor%20Object%20Reference) (OtherComp :type Primitive%20Component%20Object%20Reference) (OtherBodyIndex :type Integer) (bFromSweep :type Boolean) (SweepResult :type Hit%20Result%20Structure%20%28by%20ref%29))
  (bind _returnvalue (Game|GetPlayerController 0))
  (bind _ascart_pawn (Utilities|Casting|CastToCartPawn OtherActor))
  (Utilities|FlowControl|DoOnce false
    (:Completed
      (Variables|/Script/Engine.SpringArmComponent|SetCameraLagSpeed (Variables|/Game/Prog/Blueprints/Character/CartPawn.CartPawn_C|GetSpringArm _ascart_pawn) 0.001)
      (bind _returnvalue_2 (UserInterface|CreateWidget "/Game/Prog/Widgets/WG_EndGame.WG_EndGame_C" 0 (Variables|Default|Getwin?)))
      (UserInterface|Viewport|AddtoViewport _returnvalue_2 0)
      (Variables|/Game/Prog/Blueprints/Character/CartPawn.CartPawn_C|SetCartSpeed _ascart_pawn 1e+02)
      (Input|SetInputModeUIOnly _returnvalue _returnvalue_2 "DoNotLock")
      (Variables|/Script/Engine.PlayerController|SetbShowMouseCursor _returnvalue true))))

(event EventBeginPlay)

(event Collision|EventActorBeginOverlap
  (params (OtherActor :type Actor%20Object%20Reference)))

(event EventTick
  (params (DeltaSeconds :type Float%20%28single-precision%29)))

(fn ConstructionScript)