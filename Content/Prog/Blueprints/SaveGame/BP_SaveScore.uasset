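; BP_SaveScore holds a high-score table as parallel Scores and Names arrays, apparently for the save game.
; AddPlayer appends an entry unsorted, and GetPlayer returns the score and name at an index.
; SortTabs runs an insertion sort by descending score, moving names in step with scores.
; CleanTab sorts, then resizes both arrays to nine entries, which trims the lowest scores or pads shorter tables.
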(fn SortTabs
  (bind _scores (Variables|Default|GetScores))
  (bind _names (Variables|Default|GetNames))
  (for _index (range 1 (Utilities|Array|LastIndex (Variables|Default|GetScores)))
    (LocalVariables|Setj (- _index 1))
    (LocalVariables|SetKeyScore (Utilities|Array|Get(acopy) (Variables|Default|GetScores) _index))
    (LocalVariables|SetKeyName (Utilities|Array|Get(acopy) (Variables|Default|GetNames) _index))
    (while (and (>= (LocalVariables|Getj) 0) (< (Utilities|Array|Get(acopy) (Variables|Default|GetScores) (LocalVariables|Getj)) (LocalVariables|GetKeyScore)))
      (Utilities|Array|SetArrayElem _scores (+ (LocalVariables|Getj) 1) (Utilities|Array|Get(acopy) _scores (LocalVariables|Getj)))
      (Utilities|Array|SetArrayElem _names (+ (LocalVariables|Getj) 1) (Utilities|Array|Get(acopy) _names (LocalVariables|Getj)))
      (Math|Integer|DecrementInt (LocalVariables|Getj)))
    (Utilities|Array|SetArrayElem (Variables|Default|GetScores) (+ (LocalVariables|Getj) 1) (LocalVariables|GetKeyScore))
    (Utilities|Array|SetArrayElem (Variables|Default|GetNames) (+ (LocalVariables|Getj) 1) (LocalVariables|GetKeyName))))

(fn GetPlayer
  (params (Index :type Integer))
  (return (Utilities|Array|Get(acopy) (Variables|Default|GetScores) Index) (Utilities|Array|Get(acopy) (Variables|Default|GetNames) Index)))

(fn AddPlayer
  (params (Score :type Integer) (Name :type Text))
  (Utilities|Array|Add (Variables|Default|GetScores) Score)
  (Utilities|Array|Add (Variables|Default|GetNames) Name))

(fn CleanTab
  (CallFunction|SortTabs)
  (Utilities|Array|Resize (Variables|Default|GetScores) 9)
  (Utilities|Array|Resize (Variables|Default|GetNames) 9))