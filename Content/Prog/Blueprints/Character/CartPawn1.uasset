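; Cart pawn that rides one of two rail splines and jumps between them on Space Bar.
; A timeline drives progress along the active spline, with play rate eased by tangent slope so descents run faster.
; Each update re-anchors a bridge spline between both rails at the current progress.
; A second timeline, played forward or reversed, moves the cart across that bridge while blending rotation, then swaps the active rail.
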(event EventBeginPlay
  (bind _timeline_0 (Variables|Default|GetTimeline_0))
  (bind _spline (Variables|Default|GetSpline))
  (bind _spline2 (Variables|Spline|GetSpline2))
  (bind _spline1 (Variables|Spline|GetSpline1))
  (bind _spline_2 (Variables|/Game/Prog/Blueprints/RailActor.RailActor_C|GetSpline _spline2))
  (bind _spline_3 (Variables|/Game/Prog/Blueprints/RailActor.RailActor_C|GetSpline _spline1))
  (Variables|Default|SetActiveSpline (Variables|Spline|GetSpline1))
  (bind _spline_4 (Timeline|Timeline_0 Play)
    (:Update
      (Variables|Default|SetValueTimeline _spline_4)
      (Utilities|FlowControl|Sequence
        (:then_0
          ;[1 1 1] SplineBetweenRailway
          (Spline|SetLocationatSplinePoint _spline 0 (.location (Spline|GetTransformatDistanceAlongSpline _spline_3 (* (Variables|Default|GetValueTimeline) (Spline|GetSplineLength _spline_3)) "World" false)) "World" true)
          (Spline|SetLocationatSplinePoint _spline 1 (.location (Spline|GetTransformatDistanceAlongSpline _spline_2 (* (Variables|Default|GetValueTimeline) (Spline|GetSplineLength _spline_2)) "World" false)) "World" true))
        (:then_1
          ;[1 1 1] CartLocation/Rotation
          (if (not (Variables|Default|Getswitching?))
            (Transformation|SetActorRotation (.rotation (Spline|GetTransformatDistanceAlongSpline (Variables|/Game/Prog/Blueprints/RailActor.RailActor_C|GetSpline (Variables|Default|GetActiveSpline)) (* (Spline|GetSplineLength (Variables|/Game/Prog/Blueprints/RailActor.RailActor_C|GetSpline (Variables|Default|GetActiveSpline))) (Variables|Default|GetValueTimeline)) "World" false)))
            (Transformation|SetActorLocation (+ (.location (Spline|GetTransformatDistanceAlongSpline (Variables|/Game/Prog/Blueprints/RailActor.RailActor_C|GetSpline (Variables|Default|GetActiveSpline)) (* (Spline|GetSplineLength (Variables|/Game/Prog/Blueprints/RailActor.RailActor_C|GetSpline (Variables|Default|GetActiveSpline))) (Variables|Default|GetValueTimeline)) "World" false)) "0, 0,25.000000") false false)))
        (:then_2
          ;[1 1 1] CartPlayRate
          (Components|Timeline|SetPlayRate _timeline_0 (Math|Interpolation|FInterpTo (Components|Animation|GetPlayRate _timeline_0) (Math|Float|MapRangeClamped (.z (Spline|GetTangentatDistanceAlongSpline (Variables|/Game/Prog/Blueprints/RailActor.RailActor_C|GetSpline (Variables|Default|GetActiveSpline)) (* (Spline|GetSplineLength (Variables|/Game/Prog/Blueprints/RailActor.RailActor_C|GetSpline (Variables|Default|GetActiveSpline))) (Variables|Default|GetValueTimeline)) "Local")) -1.4e+03 1.4e+03 7.2 0.8) (Utilities|Time|GetWorldDeltaSeconds) 1.2)))))))

(event Input|KeyboardEvents|SpaceBar
  (params (Key :type Key%20Structure :default "None"))
  (bind _valuetimeline (Variables|Default|GetValueTimeline))
  (bind _spline (Variables|Default|GetSpline))
  (bind _spline1 (Variables|Spline|GetSpline1))
  (bind _spline2 (Variables|Spline|GetSpline2))
  (bind _spline_2 (Variables|/Game/Prog/Blueprints/RailActor.RailActor_C|GetSpline _spline2))
  (bind _spline_3 (Variables|/Game/Prog/Blueprints/RailActor.RailActor_C|GetSpline _spline1))
  ;[1 1 1] SwitchRail => TODO Add UpPoint on Spline
  (:Pressed
    (if (not (Variables|Default|Getswitching?))
      (Variables|Default|Setswitching? true)
      (if (== (Variables|Default|GetActiveSpline) (Variables|Spline|GetSpline1))
        (bind _newtrack_0 (Timeline|SwitchRail Play)
          (:Update
            (Transformation|SetActorLocationAndRotation (+ (.location (Spline|GetTransformatDistanceAlongSpline _spline (* _newtrack_0 (Spline|GetSplineLength _spline)) "World" false)) "0,0.000000,25.000000") (Math|Interpolation|Ease "Linear" _newtrack_0 (.rotation (Spline|GetTransformatDistanceAlongSpline _spline_3 (* _valuetimeline (Spline|GetSplineLength _spline_3)) "World" false)) (.rotation (Spline|GetTransformatDistanceAlongSpline _spline_2 (* _valuetimeline (Spline|GetSplineLength _spline_2)) "World" false)) true)))
          (:Finished
            (Variables|Default|Setswitching? false)
            (Variables|Default|SetActiveSpline (select (== (Variables|Default|GetActiveSpline) (Variables|Spline|GetSpline1)) (Variables|Spline|GetSpline2) (Variables|Spline|GetSpline1)))))
        (else
          (Timeline|SwitchRail Reverse))))))

(fn ConstructionScript
  (Variables|/Script/Engine.SpringArmComponent|SetTargetArmLength (Variables|Default|GetSpringArm) (Variables|Camera|GetCameraDistance)))

(fn AdjustCamera
  (params (DeltaTime :type Float%20%28single-precision%29) (InterpSpeed :type Float%20%28single-precision%29))
  (bind _springarm (Variables|Default|GetSpringArm))
  (Variables|/Script/Engine.SpringArmComponent|SetTargetArmLength _springarm (Math|Interpolation|FInterpTo (Variables|/Script/Engine.SpringArmComponent|GetTargetArmLength _springarm) (Variables|Camera|GetCameraDistance) DeltaTime InterpSpeed)))