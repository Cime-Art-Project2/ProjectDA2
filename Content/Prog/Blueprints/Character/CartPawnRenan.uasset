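; Cart pawn prototype that switches between a rail below and a rail above through Jump and GoDown input.
; Each tick, vertical traces cache both rail actors, then SplineToUse picks which timeline drives actor X toward that spline's end, gated by DoOnce nodes.
; Jump animates mesh height and selects the upper rail if found; GoDown selects the lower.
; Slope-momentum rail movement, gravity and camera helpers are defined but uncalled here.
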(event EventTick
  (params (DeltaSeconds :type Float%20%28single-precision%29))
  (bind _returnvalue (Transformation|GetActorLocation))
  (bind _returnvalue_2 (Transformation|GetActorLocation))
  (bind _spline2 (Variables|Default|GetSpline2))
  (bind _spline1 (Variables|Default|GetSpline1))
  (bind _spline (Variables|/Game/Prog/Blueprints/RailActorRenan.RailActorRenan_C|GetSpline _spline1))
  (bind _spline_2 (Variables|/Game/Prog/Blueprints/RailActorRenan1.RailActorRenan1_C|GetSpline _spline2))
  (Utilities|FlowControl|Sequence
    (:then_0
      (Utilities|Raycast))
    (:then_1
      (switch int (Variables|Default|GetSplineToUse)
        (:Default
          (Development|PrintString "Spline1" :!label _label)
          (Utilities|FlowControl|Sequence
            (:then_0
              (bind _newtrack_0 (Timeline|Timeline_3 Stop)
                (:Update
                  (Components|Timeline|SetPlayRate (Variables|Default|GetTimeline_3) 0.2)
                  (Transformation|SetActorLocation (Math|Vector|MakeVector (* _newtrack_0 (.x (Spline|GetLocationatDistanceAlongSpline _spline_2 (Spline|GetSplineLength _spline_2) "World"))) (.y _returnvalue) (.z _returnvalue)) false false))))
            (:then_1
              (goto _label_3 Reset))
            (:then_2
              (Utilities|FlowControl|DoOnce false :!label _label_2
                (:Completed
                  (bind _newtrack_0_2 (Timeline|Timeline_2 Play)
                    (:Update
                      (Components|Timeline|SetPlayRate (Variables|Default|GetTimeline_2) 0.2)
                      (Transformation|SetActorLocation (Math|Vector|MakeVector (* _newtrack_0_2 (.x (Spline|GetLocationatDistanceAlongSpline _spline (Spline|GetSplineLength _spline) "World"))) (.y _returnvalue_2) (.z _returnvalue_2)) false false))))))))
        (:1
          (goto _label))
        (:2
          (Development|PrintString "Spline2")
          (Utilities|FlowControl|Sequence
            (:then_0
              (goto _label_2 Reset))
            (:then_1
              (Timeline|Timeline_2 Stop))
            (:then_2
              (Utilities|FlowControl|DoOnce false :!label _label_3
                (:Completed
                  (Timeline|Timeline_3 Play))))))))))

(event Input|ActionEvents|InputActionGoDown
  (params (Key :type Key%20Structure :default "None"))
  (:Pressed
    (if (Utilities|IsValid (Variables|Default|GetSpline1))
      (Variables|Default|SetSplineToUse 1))))

(event Input|ActionEvents|InputActionJump
  (params (Key :type Key%20Structure :default "None"))
  (:Pressed
    (if (Variables|Default|GetCanJump?)
      (Variables|Default|SetCanJump? false)
      (bind _newtrack_0 (Timeline|Timeline_0 PlayFromStart)
        (:Update
          (Transformation|SetRelativeLocation (Variables|Default|GetSkeletalMesh) (Math|Vector|MakeVector 0.0 0.0 (- (* _newtrack_0 (Variables|Default|GetJumpHeigh)) 3e+01)) false false)
          (if (and (Utilities|IsValid (Variables|Default|GetSpline2)) (Math|Boolean|Equal(Boolean) (Variables|Default|GetCanJump?) false))
            (Variables|Default|SetSplineToUse 2)))
        (:Finished
          (Variables|Default|SetCanJump? true))))))

(fn ConstructionScript
  (Variables|/Script/Engine.SpringArmComponent|SetTargetArmLength (Variables|Default|GetSpringArm) (Variables|Camera|GetCameraDistance)))

(fn ConsumeVelocity
  (params (DeltaTime :type Float%20%28single-precision%29))
  (LocalVariables|SetCurLoc (Transformation|GetActorLocation))
  (Variables|Physics|SetCartVelocity (Math|Vector|SelectVector "0, 0, 0" (+ (Variables|Physics|GetCartVelocity) (* (Variables|Physics|GetGravityDirection) (* DeltaTime (Variables|Physics|GetGravityForce)))) (Utilities|IsValid 0)))
  (Transformation|SetActorLocation (+ (Transformation|GetActorLocation) (* (Variables|Physics|GetCartVelocity) DeltaTime)) true false))

(fn AdjustCamera
  (params (DeltaTime :type Float%20%28single-precision%29) (InterpSpeed :type Float%20%28single-precision%29))
  (bind _springarm (Variables|Default|GetSpringArm))
  (Variables|/Script/Engine.SpringArmComponent|SetTargetArmLength _springarm (Math|Interpolation|FInterpTo (Variables|/Script/Engine.SpringArmComponent|GetTargetArmLength _springarm) (Variables|Camera|GetCameraDistance) DeltaTime InterpSpeed)))

(fn StopMovement
  (params (StopGravity :type Boolean))
  (Variables|Physics|SetCartVelocity "0, 0, 0")
  (Variables|Physics|SetGravityForce (Math|Float|SelectFloat 0.0 2.0 StopGravity)))

(fn MoveonSpline
  (params (RailSpline :type Rail%20Actor%20Object%20Reference))
  (bind (_location _locationwithoffset _tangent _upvector) (Default|GetRailData RailSpline "World"))
  (bind _cartspeed (Variables|Physics|GetCartSpeed))
  (bind _returnvalue (Math|Vector|Normalize _tangent))
  (bind _returnvalue_2 (/ _cartspeed 1e+02))
  (Variables|Physics|SetTangentZ (Math|Interpolation|FInterpTo (Variables|Physics|GetTangentZ) (.z _returnvalue) (Utilities|Time|GetWorldDeltaSeconds) (Math|Float|SelectFloat 5.0 2.5 (< (.z _returnvalue) 0.0))))
  (Variables|Physics|SetMomentumSpeed (Math|Interpolation|FInterpTo (Variables|Physics|GetMomentumSpeed) (Math|Float|MapRangeClamped (Variables|Physics|GetTangentZ) -1.0 1.0 (* _returnvalue_2 1.6) (* _returnvalue_2 0.4)) (Utilities|Time|GetWorldDeltaSeconds) 5.0))
  (Transformation|SetActorLocation (+ _locationwithoffset (* _tangent (* (/ (Math|Interpolation|FInterpTo (Variables|Physics|GetMomentumSpeed) (Math|Float|MapRangeClamped (Variables|Physics|GetTangentZ) -1.0 1.0 (* _returnvalue_2 1.6) (* _returnvalue_2 0.4)) (Utilities|Time|GetWorldDeltaSeconds) 5.0) (Variables|Physics|GetCartFriction)) (Utilities|Time|GetWorldDeltaSeconds)))) false true)
  (Transformation|SetActorRotation (Math|Rotator|MakeRotfromXZ _tangent _upvector)))

(fn GetCartSpeed
  (return (* (Variables|Physics|GetMomentumSpeed) 1e+02)))