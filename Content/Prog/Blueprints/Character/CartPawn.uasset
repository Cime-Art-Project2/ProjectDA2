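; Player cart pawn that rides spline-based RailActors and can jump, switch to a linked rail or drop toward one below.
; Tick integrates a manual velocity, from the rail tangent or gravity when airborne, then snaps attached carts to the spline with slope-driven momentum.
; Rail switches follow a timeline arc after distance and height checks.
; Jumps keep the previous rail for alignment until a falling cart enters a rail.
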(event Custom|OnEnterRail
  (params (Rail :type Rail%20Actor%20Object%20Reference))
  (if (< (.z (Variables|Physics|GetCartVelocity)) 0.0)
    (Variables|Spline|SetPreviousAttachedSpline 0)
    (bind _output_get (Variables|Spline|SetAttachedSpline Rail))
    (Physics|StopMovement false)
    (Transformation|SetActorLocation (.LocationWithOffset (Default|GetRailData _output_get "World")) false true)
    (if (Variables|Physics|GetJumping)
      (Variables|Physics|SetJumping false))))

(event Custom|OnReachedRailEnd
  (params (ExitVelocity :type Vector))
  (Utilities|IsValid (Variables|Spline|GetAttachedSpline)
    (:Is%20Valid
      (Variables|Spline|SetPreviousAttachedSpline 0)
      (Variables|Spline|SetAttachedSpline 0)
      (Variables|Physics|SetCartVelocity ExitVelocity))))

(event EventBeginPlay
  (Variables|Physics|SetCartVelocity (* (Transformation|GetActorForwardVector) (Variables|Physics|GetCartSpeed))))

(event EventTick
  (params (DeltaSeconds :type Float%20%28single-precision%29))
  (bind _returnvalue (Transformation|GetActorLocation))
  (bind _attachedspline (Variables|Spline|GetAttachedSpline))
  (Development|PrintString (Utilities|String|Append (Utilities|GetDisplayName (Variables|Spline|GetAttachedSpline)) " -- " (Utilities|GetDisplayName (Variables|Spline|GetPreviousAttachedSpline))) true true "(R=0.000000,G=0.660000,B=1.000000,A=1.000000)" DeltaSeconds)
  (Development|PrintString (Utilities|String|Append "Velocity : " (Utilities|String|ToString(Vector) (Variables|Physics|GetCartVelocity))) true true "(R=1.000000,G=0.523420,B=0.000000,A=1.000000)" DeltaSeconds)
  (Components|Timeline|SetPlayRate (Variables|Default|GetSkeletalMesh) (/ (Physics|GetCartSpeed) 1e+02))
  (Physics|ConsumeVelocity DeltaSeconds)
  (CallFunction|AdjustCamera DeltaSeconds 4.0)
  (Utilities|IsValid _attachedspline
    (:Is%20Valid
      (Physics|MoveonSpline _attachedspline)
      (Variables|/Script/Engine.SpringArmComponent|SetTargetOffset (Variables|Default|GetSpringArm) (* (Transformation|GetActorForwardVector) (Variables|/Game/Prog/Blueprints/Bp_CartPlayerController.Bp_CartPlayerController_C|GetOffSet (.AsBp%20Cart%20Player%20Controller (Utilities|Casting|CastToBp_CartPlayerController (Game|GetPlayerController 0)))))))
    (:Is%20Not%20Valid
      (Utilities|IsValid (Variables|Spline|GetPreviousAttachedSpline)
        (:Is%20Valid
          (Transformation|SetActorRotation (Math|Interpolation|RInterpTo (Transformation|GetActorRotation) (.Rotation (Default|GetRailData (Variables|Spline|GetPreviousAttachedSpline) "World")) (Utilities|Time|GetWorldDeltaSeconds) 5.0))
          (if (Variables|Physics|GetJumping)
            (Transformation|SetActorLocation (Math|Vector|MakeVector (.x _returnvalue) (.y (Spline|FindLocationClosesttoWorldLocation (Variables|/Game/Prog/Blueprints/RailActor.RailActor_C|GetSpline (Variables|Spline|GetPreviousAttachedSpline)) (Transformation|GetActorLocation) "World")) (.z _returnvalue)) false false)))
        (:Is%20Not%20Valid
          (Transformation|SetActorRotation (Math|Interpolation|RInterpTo (Transformation|GetActorRotation) (Math|Conversions|RotationFromXVector (Math|Vector|Normalize (CallFunction|GetCartVelocity))) (Utilities|Time|GetWorldDeltaSeconds) 4.0)))))))

(event Custom|SwitchRail
  (params (Height :type Float%20%28single-precision%29) (Distance :type Float%20%28single-precision%29) (PreviousLocation :type Vector) (TargetLocation :type Vector))
  ;[1 0 0 1 11] Mettre AttachedSpline sur null impact PreviousAttachedSpline ce qui empeche certaine instructions d'être éxecuté correctement...
  (Variables|Spline|SetPreviousAttachedSpline (.Copy (Utilities|AdvancedGet (Variables|Spline|GetAttachedSpline))))
  (Collision|SetCollisionEnabled (Variables|/Game/Prog/Blueprints/RailActor.RailActor_C|GetCartReceiver (Variables|Spline|GetAttachedSpline)) "NoCollision")
  (Variables|Spline|SetAttachedSpline 0)
  (bind (_direction _alpha _up) (Timeline|Timeline_0 PlayFromStart)
    (:Update
      (Transformation|SetActorLocation (+ (Math|Vector|Lerp(Vector) PreviousLocation TargetLocation _alpha) (Math|Vector|MakeVector 0.0 0.0 (* _up Height))) false true))
    (:Finished
      (Variables|Spline|SetAttachedSpline (Variables|/Game/Prog/Blueprints/RailActor.RailActor_C|GetTargetSwitchRail (Variables|Spline|GetPreviousAttachedSpline)))
      (Collision|SetCollisionEnabled (Variables|/Game/Prog/Blueprints/RailActor.RailActor_C|GetCartReceiver (Variables|Spline|GetPreviousAttachedSpline)) "QueryOnly"))))

(event Input|ActionEvents|InputActionGoDown
  (params (Key :type Key%20Structure :default "None"))
  (bind _returnvalue (Transformation|GetActorLocation))
  (:Pressed
    (Utilities|IsValid (Variables|Spline|GetAttachedSpline)
      (:Is%20Valid
        (Variables|Physics|SetCartVelocity (- (.Tangent (Default|GetRailData (Variables|Spline|GetAttachedSpline) "World")) "0, 0,980.000000"))
        (bind (_outhit _returnvalue_2) (Collision|SphereTraceForObjects _returnvalue (- (+ _returnvalue (* (Transformation|GetActorForwardVector) (Math|Vector|VectorLength (CallFunction|GetCartVelocity)))) "0, 0,5000.000000") 64.0 (Utilities|Array|MakeArray "ObjectTypeQuery7") true (Utilities|Array|MakeArray (Variables|Spline|GetAttachedSpline)) "None"))
        (if _returnvalue_2
          (bind _asrail_actor (Utilities|Casting|CastToRailActor (.HitActor (Collision|BreakHitResult _outhit))))
          (Variables|Spline|SetAttachedSpline 0)
          (Variables|Spline|SetPreviousAttachedSpline _asrail_actor)
          (Collision|SetCollisionEnabled (Variables|Default|GetCharacterHitbox) "NoCollision")
          (Utilities|FlowControl|RetriggerableDelay 0.25)
          (Collision|SetCollisionEnabled (Variables|Default|GetCharacterHitbox) "QueryAndPhysics"))))))

(event Input|ActionEvents|InputActionJump
  (params (Key :type Key%20Structure :default "None"))
  (bind _cartspeed (Variables|Physics|GetCartSpeed))
  (bind _returnvalue (/ _cartspeed 1e+02))
  (:Pressed
    (Utilities|IsValid (Variables|Spline|GetAttachedSpline)
      (:Is%20Valid
        (if (<= (Math|Float|Absolute(Float) (.z (Math|Vector|Normalize (.Tangent (Default|GetRailData (Variables|Spline|GetAttachedSpline) "World"))))) 0.55)
          (Physics|StopMovement false)
          (Variables|Physics|SetCartVelocity (Math|Vector|MakeVector (.x (* (.Tangent (Default|GetRailData (Variables|Spline|GetAttachedSpline) "World")) (* _returnvalue 0.25))) (.y (* (.Tangent (Default|GetRailData (Variables|Spline|GetAttachedSpline) "World")) (* _returnvalue 0.25))) (* _returnvalue (* (.z (Variables|Physics|GetGravityDirection)) -0.35))))
          (Variables|Spline|SetPreviousAttachedSpline (Variables|Spline|GetAttachedSpline))
          (Variables|Spline|SetAttachedSpline 0)
          (Variables|Physics|SetJumping true))))))

(event Input|ActionEvents|InputActionSwitchRail
  (params (Key :type Key%20Structure :default "None"))
  (bind _returnvalue (Transformation|GetActorLocation))
  (bind _returnvalue_2 (Transformation|GetActorForwardVector))
  (bind _cartvelocity (Variables|Physics|GetCartVelocity))
  (bind _attachedspline (Variables|Spline|GetAttachedSpline))
  (bind _returnvalue_3 (* _cartvelocity _returnvalue_2))
  (bind _targetswitchrail (Variables|/Game/Prog/Blueprints/RailActor.RailActor_C|GetTargetSwitchRail _attachedspline))
  (bind _returnvalue_4 (+ _returnvalue _returnvalue_3))
  (bind _spline (Variables|/Game/Prog/Blueprints/RailActor.RailActor_C|GetSpline _targetswitchrail))
  (bind _returnvalue_5 (Spline|FindLocationClosesttoWorldLocation _spline _returnvalue_4 "World"))
  (bind _z (Math|Vector|BreakVector _returnvalue_4))
  (bind _z_2 (Math|Vector|BreakVector _returnvalue_5))
  (bind _returnvalue_6 (- _z _z_2))
  (bind _returnvalue_7 (Math|Float|Absolute(Float) _returnvalue_6))
  (:Pressed
    (if (and (<= (Math|Vector|Distance(Vector) _returnvalue_4 _returnvalue_5) (Variables|Gameplay|RailSwitch|GetMaxDistanceToSwitch)) (<= _returnvalue_7 (Variables|Gameplay|RailSwitch|GetMaxHeightToSwitch)))
      (CallFunction|SwitchRail _returnvalue_7 0.0 (Transformation|GetActorLocation) _returnvalue_5)
      (else
        (Development|PrintString "Can't Switch !" true true "(R=1.000000,G=0.153407,B=0.113603,A=1.000000)")))))

(fn ConstructionScript
  (Variables|/Script/Engine.SpringArmComponent|SetTargetArmLength (Variables|Default|GetSpringArm) (Variables|Camera|GetCameraDistance)))

(fn ConsumeVelocity
  (params (DeltaTime :type Float%20%28single-precision%29))
  (LocalVariables|SetCurLoc (Transformation|GetActorLocation))
  (Variables|Spline|GetAttachedSpline
    (:then
      (Variables|Physics|SetCartVelocity (.Tangent (Default|GetRailData (Variables|Spline|GetAttachedSpline) "World"))))
    (:else
      (Variables|Physics|SetCartVelocity (+ (Variables|Physics|GetCartVelocity) (* (Variables|Physics|GetGravityDirection) (* DeltaTime (Variables|Physics|GetGravityForce)))))))
  (Transformation|SetActorLocation (+ (Transformation|GetActorLocation) (* (Variables|Physics|GetCartVelocity) DeltaTime)) true false))

(fn AdjustCamera
  (params (DeltaTime :type Float%20%28single-precision%29) (InterpSpeed :type Float%20%28single-precision%29))
  (bind _springarm (Variables|Default|GetSpringArm))
  (Variables|/Script/Engine.SpringArmComponent|SetTargetArmLength _springarm (Math|Interpolation|FInterpTo (Variables|/Script/Engine.SpringArmComponent|GetTargetArmLength _springarm) (Variables|Camera|GetCameraDistance) DeltaTime InterpSpeed)))

(fn StopMovement
  (params (StopGravity :type Boolean))
  (Variables|Physics|SetCartVelocity "0, 0, 0")
  (Variables|Physics|SetGravityForce (Math|Float|SelectFloat 0.0 2.0 StopGravity)))

(fn MoveonSpline
  (params (RailSpline :type Rail%20Actor%20Object%20Reference))
  (bind (_location _locationwithoffset _tangent _upvector) (Default|GetRailData RailSpline "World"))
  (bind _cartspeed (Variables|Physics|GetCartSpeed))
  (bind _returnvalue (Math|Vector|Normalize _tangent))
  (bind _returnvalue_2 (/ _cartspeed 1e+02))
  (Variables|Physics|SetTangentZ (Math|Interpolation|FInterpTo (Variables|Physics|GetTangentZ) (.z _returnvalue) (Utilities|Time|GetWorldDeltaSeconds) (Math|Float|SelectFloat 5.0 2.5 (< (.z _returnvalue) 0.0))))
  (Variables|Physics|SetMomentumSpeed (Math|Interpolation|FInterpTo (Variables|Physics|GetMomentumSpeed) (Math|Float|MapRangeClamped (Variables|Physics|GetTangentZ) -1.0 1.0 (* _returnvalue_2 1.6) (* _returnvalue_2 0.4)) (Utilities|Time|GetWorldDeltaSeconds) 5.0))
  (Transformation|SetActorLocation (+ _locationwithoffset (* _tangent (* (/ (Math|Interpolation|FInterpTo (Variables|Physics|GetMomentumSpeed) (Math|Float|MapRangeClamped (Variables|Physics|GetTangentZ) -1.0 1.0 (* _returnvalue_2 1.6) (* _returnvalue_2 0.4)) (Utilities|Time|GetWorldDeltaSeconds) 5.0) (Variables|Physics|GetCartFriction)) (Utilities|Time|GetWorldDeltaSeconds)))) false true)
  (Transformation|SetActorRotation (Math|Rotator|MakeRotfromXZ _tangent _upvector)))

(fn GetCartSpeed
  (return (* (Variables|Physics|GetMomentumSpeed) 1e+02)))