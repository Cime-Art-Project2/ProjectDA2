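; A placeable trigger volume that changes the camera distance of any CartPawn entering its box.
; Begin overlap copies the Y component of its CameraDistance vector to the pawn, and end overlap optionally restores a hardcoded default.
; The construction script sizes the box, constrains the vector to local Y and redraws a temporary debug line previewing the distance, flushing existing persistent debug lines first.
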(event OnComponentBeginOverlap(Box)
  (params (OverlappedComponent :type Primitive%20Component%20Object%20Reference) (OtherActor :type Actor%20Object%20Reference) (OtherComp :type Primitive%20Component%20Object%20Reference) (OtherBodyIndex :type Integer) (bFromSweep :type Boolean) (SweepResult :type Hit%20Result%20Structure%20%28by%20ref%29))
  (bind _ascart_pawn (Utilities|Casting|CastToCartPawn OtherActor))
  (Variables|/Game/Prog/Blueprints/Character/CartPawn.CartPawn_C|SetCameraDistance _ascart_pawn (.y (Variables|Default|GetCameraDistance))))

(event OnComponentEndOverlap(Box)
  (params (OverlappedComponent :type Primitive%20Component%20Object%20Reference) (OtherActor :type Actor%20Object%20Reference) (OtherComp :type Primitive%20Component%20Object%20Reference) (OtherBodyIndex :type Integer))
  (if (Variables|Default|GetResetDistanceOnExit)
    (bind _ascart_pawn (Utilities|Casting|CastToCartPawn OtherActor))
    (Variables|/Game/Prog/Blueprints/Character/CartPawn.CartPawn_C|SetCameraDistance _ascart_pawn 8e+02)))

(fn ConstructionScript
  (Components|Box|SetBoxExtent (Variables|Default|GetBox) (Variables|Default|GetBoxSize) true)
  (Variables|Default|SetCameraDistance (Math|Vector|MakeVector 0.0 (.y (Variables|Default|GetCameraDistance)) 0.0))
  (Rendering|Debug|FlushPersistentDebugLines)
  (Rendering|Debug|DrawDebugLine (Transformation|GetActorLocation) (Math|Transform|TransformLocation (Transformation|GetActorTransform) (Variables|Default|GetCameraDistance)) "(R=0.000000,G=1.000000,B=0.322387,A=1.000000)" 5.0 0.0))